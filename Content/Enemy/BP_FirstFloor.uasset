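; First-floor enemy, configured from a DT_Enemys row, that tracks perceived actors and damages the player.
; Construction loads mesh and life bar by Type, while BeginPlay looks up RowName, setting mesh and life values and passing the widget to SetWindowTitleBarState.
; AI perception writes the sensed actor to the blackboard target, clearing it otherwise.
; Overlapping Box_Damage makes BP_FirstPersonCharacter lose life by the row's damage.
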(event `self.ReceiveBeginPlay`
  ;[1 1 1] prueba
  (bind _returnvalue (`|GetDataTableRow` "/Game/Enemy/DT_Enemys.DT_Enemys" (`self.Row Name`))
    (:`then`
      (bind _output_get (set `self.EnemyData` _returnvalue))
      (bind (_maxlife _damage _mesh _currentlife) (break `/Game/Enemy/FEnemy` _output_get))
      (`SkinnedMeshComponent.SetSkinnedAssetAndUpdate` (`self.Mesh`) _mesh true)
      (bind _aswbp_enemy_life_bar (cast `/Game/Enemy/WBP_EnemyLifeBar` (`WidgetComponent.GetWidget` (`self.Widget`))))
      (`WidgetBlueprintLibrary.SetWindowTitleBarState` _aswbp_enemy_life_bar "Overlay")
      (set `self.Current Life` _currentlife)
      (set `self.Max Life` _maxlife))))

(event `self.AIPerception.OnTargetPerceptionUpdated`
  (params (Actor :type "Actor Object Reference") (Stimulus :type "AIStimulus Structure"))
  (`BlackboardComponent.SetValueAsObject` (`AIBlueprintHelperLibrary.GetBlackboard` (`self.GetController`)) (`self.TargetKey`) (select `bool` (`.bSuccessfullySensed` (break `AIStimulus` Stimulus)) :`true` Actor :!type "Object Object Reference")))

(event `self.Box_Damage.OnComponentBeginOverlap`
  (params (OverlappedComponent :type "PrimitiveComponent Object Reference") (OtherActor :type "Actor Object Reference") (OtherComp :type "PrimitiveComponent Object Reference") (OtherBodyIndex :type Integer) (bFromSweep :type Boolean) (SweepResult :type "HitResult Structure (by ref)"))
  (bind _asbp_first_person_character (cast `/Game/FirstPerson/Blueprints/BP_FirstPersonCharacter` OtherActor))
  (`/Game/FirstPerson/Blueprints/BP_FirstPersonCharacter.LoseLife` _asbp_first_person_character (`.Damage_8_749E09834C9BD1D39980DB86AF692E69` (break `/Game/Enemy/FEnemy` (`self.EnemyData`)))))

(fn `LoadValues`
  (bind _returnvalue (`|GetDataTableRow` "/Game/Enemy/DT_Enemys.DT_Enemys" (`KismetStringLibrary.Conv_StringToName` (`KismetStringLibrary.Conv_ByteToString` (`self.Type`))))
    (:`then`
      (bind _output_get (set `self.EnemyData` _returnvalue))
      (bind (_maxlife _damage _mesh _currentlife) (break `/Game/Enemy/FEnemy` _output_get))
      (`SkinnedMeshComponent.SetSkinnedAssetAndUpdate` (`self.Mesh`) _mesh true)
      (bind _aswbp_enemy_life_bar (cast `/Game/Enemy/WBP_EnemyLifeBar` (`WidgetComponent.GetWidget` (`self.Widget`))))
      (`/Game/Enemy/WBP_EnemyLifeBar.UpdateLifeBar` _aswbp_enemy_life_bar _currentlife _maxlife))))

(fn `UserConstructionScript`
  (`self.LoadValues`))