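; Damageable actor component that gives enemies a life pool and destroys the owner when it runs out.
; It resets current life to the maximum on BeginPlay.
; GetDamage subtracts incoming damage, broadcasts an on-life-change dispatcher with the new and maximum values, then calls Death if life is no longer above zero.
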(event `self.ReceiveBeginPlay`
  (set `self.CurrentLife` (`self.MaxLife`)))

(fn `Death`
  (`Actor.K2_DestroyActor` (`self.GetOwner`)))

(fn `GetDamage`
  (params (InDamage :type "Float (double-precision)"))
  (set `self.CurrentLife` (- (`self.CurrentLife`) InDamage))
  (`self.OnlifeChange` (`self.CurrentLife`) (`self.MaxLife`))
  (if (not (`self.IsAlive`))
    (`self.Death`)))

(fn `IsAlive`
  (returns (IsAlive :type Boolean))
  (return (> (`self.CurrentLife`) 0.0)))