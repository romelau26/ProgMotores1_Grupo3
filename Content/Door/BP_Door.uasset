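; BP_Door is a door actor that slides smoothly between its starting location and an offset open position.
; OpenDoorSmooth plays the MoveDoor timeline at a rate derived from TimeToOpen, lerping from the location cached at BeginPlay toward OpenOffset.
; CloseDoorSmooth reverses the same timeline.
; When the timeline finishes, OnDoorStateChange reports open or closed based on playback direction.
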(event `self.ReceiveBeginPlay`
  (set `self.InitialLocation` (`self.K2_GetActorLocation`)))

(event `OpenDoorSmooth`
  (bind _initiallocation (`self.InitialLocation`))
  (`TimelineComponent.SetPlayRate` (`self.MoveDoor`) (/ 1.0 (`self.TimeToOpen`)))
  (bind (_direction _currenttime) (`Timeline|MoveDoor` :!label _label)
    (:`Update`
      (`self.K2_SetActorLocation` (`KismetMathLibrary.VLerp` _initiallocation (+ _initiallocation (`self.OpenOffset`)) _currenttime)))
    (:`Finished`
      (`self.OnDoorStateChange` (select `ETimelineDirection` _direction :`Forward` true)))))

(event `CloseDoorSmooth`
  (goto _label :!via `Reverse`))

(fn `UserConstructionScript`)